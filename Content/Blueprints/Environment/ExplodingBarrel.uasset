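; An explodable barrel that catches fire from fire damage, explodes after a delay or upon further fire damage, and chain-reacts with nearby barrels.
; Another barrel's blast ignites it with a short fuse, while other explosion damage detonates it immediately at a set scale.
; Explode only destroys the actor; EndPlay spawns the effect and applies scaled radial damage credited to BurnInstigator.
; The IsBurning RepNotify spawns the fire effect, which is removed on destruction.
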(event EventEndPlay
  (params (EndPlayReason :type EEndPlayReason%20Enum :default "Destroyed"))
  (bind _returnvalue (Transformation|GetActorTransform))
  (bind _explosionscale (Variables|Default|GetExplosionScale))
  (if (Utilities|Enum|Equal(Enum) EndPlayReason "Destroyed")
    (Game|SpawnActorfromClass "/Game/StarterContent/Blueprints/Blueprint_Effect_Explosion.Blueprint_Effect_Explosion_C" (Math|Transform|MakeTransform (.location _returnvalue) (.rotation _returnvalue) (* (.scale _returnvalue) (Variables|Default|GetExplosionScale))) "AlwaysSpawn" 0 0)
    (Collision|SetCollisionEnabled (Variables|Debug|GetStaticMeshComponent) "NoCollision")
    (Class|GameplayStatics|ApplyRadialDamagewithFalloff (Variables|Default|GetBaseDamage) (Variables|Default|GetMinDamage) (Transformation|GetWorldLocation (Variables|Default|GetFireLocation)) (* _explosionscale 5e+01) (* _explosionscale 1e+02) 1.2 "/Game/Blueprints/Damage/ExplosionDamage.ExplosionDamage_C" 0 self (Variables|Default|GetBurnInstigator) "ECC_Vehicle")
    (bind _fireactor (Variables|Default|GetFireActor)
      (:then
        (Actor|DestroyActor _fireactor))
      (:else
        _))
    (Actor|DestroyActor)))

(event Game|Damage|EventAnyDamage
  (params (Damage :type Float%20%28single-precision%29) (DamageType :type Damage%20Type%20Object%20Reference) (InstigatedBy :type Controller%20Object%20Reference) (DamageCauser :type Actor%20Object%20Reference))
  (Utilities|Casting|CastToFireDamage DamageType
    (:then
      (if (Variables|Default|GetisBurning)
        (bind _asexploding_barrel (Utilities|Casting|CastToExplodingBarrel DamageCauser)
          (:then
            (Variables|Default|SetBurnInstigator (Variables|ExplodingBarrel_C|GetBurnInstigator _asexploding_barrel)))
          (:CastFailed
            (Variables|Default|SetBurnInstigator 0)))
        (CallFunction|Explode)
        (else
          (Variables|Default|SetisBurning true)
          (Utilities|Time|SetTimerbyFunctionName self "Explode" (Variables|Default|GetExplosionDelay))
          (Variables|Default|SetBurnInstigator InstigatedBy))))
    (:CastFailed
      (Utilities|Casting|CastToExplosionDamage DamageType)
      (Utilities|Casting|CastToExplodingBarrel DamageCauser
        (:then
          (Variables|Default|SetisBurning true)
          (Utilities|Time|SetTimerbyFunctionName self "Explode" 0.3)
          (Variables|Default|SetBurnInstigator 0))
        (:CastFailed
          (Variables|Default|SetExplosionScale 6.0)
          (CallFunction|Explode))))))

(fn ConstructionScript)

(fn Explode
  (Actor|DestroyActor))

(fn OnRepIsBurning
  (Variables|Default|GetFireActor
    (:then)
    (:else
      (bind _returnvalue (Game|SpawnActorfromClass "/Game/StarterContent/Blueprints/Blueprint_Effect_Fire.Blueprint_Effect_Fire_C" (Transformation|GetWorldTransform (Variables|Default|GetFireLocation)) "AlwaysSpawn" 0 0))
      (Variables|Default|SetFireActor _returnvalue))))