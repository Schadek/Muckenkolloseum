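; Pistol weapon Blueprint that fires a PistolBullet when its trigger word is spoken, extending a parent weapon class.
; On attach, it runs the parent logic, then snaps to the character mesh's right-hand socket while keeping world scale.
; On the trigger word, it runs the parent logic, then always spawns the bullet just ahead of the owning character's location, using the character's rotation and setting it as owner.
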(event EventTriggerWordSpoken
  (bind _owningchar (Variables|Default|GetOwningChar))
  (|CallParentFunction)
  (Game|SpawnActorfromClass "/Game/Blueprints/Weapons/PistolBullet.PistolBullet_C" (Math|Transform|MakeTransform (+ (Transformation|GetActorLocation _owningchar) (* (Transformation|GetActorForwardVector _owningchar) 1e+01)) (Transformation|GetActorRotation _owningchar) "1,1,1") "AlwaysSpawn" _owningchar 0))

(event EventAttachtoPlayer
  (params (Char :type Muckenkolloseum%20Char%20Object%20Reference))
  (|CallParentFunction Char)
  (Transformation|AttachComponentToComponent (Variables|/Script/Engine.Character|GetMesh Char) "hand_rSocket" "SnapToTarget" "SnapToTarget" "KeepWorld" true))

(fn ConstructionScript
  (|CallParentFunction))