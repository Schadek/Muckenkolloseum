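; Voice-triggered rapid-fire weapon that snaps to the player's hand socket and blocks the owner's speech while active.
; The client trigger starts a looping timer that passes the targeted point to RapidFireTickRMI, which spawns a PistolBullet from the owner toward it.
; A grace timer starts on trigger and when speaking stops, and is cleared when speaking resumes.
; When it expires, firing stops, speech events unbind and speech is unblocked.
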(event Custom|StopRapidfire
  (bind _returnvalue (Utilities|Time|SetTimerbyEvent (delegate Custom|EndRapidFire) (Variables|Default|GetGraceperiod)))
  (Variables|Default|SetEndRapidfireHandle _returnvalue))

(event Custom|RapidFireTickRMI
  (params (LookAtDir :type Vector))
  (bind _owningchar (Variables|Default|GetOwningChar))
  (bind _returnvalue (Transformation|GetActorLocation _owningchar))
  (Game|SpawnActorfromClass "/Game/Blueprints/Weapons/PistolBullet.PistolBullet_C" (Math|Transform|MakeTransform _returnvalue (Math|Rotator|MakeRotfromX (Math|Vector|Normalize (- LookAtDir _returnvalue))) "1,1,1") "AlwaysSpawn" _owningchar _owningchar))

(event Custom|OnStartedSpeaking_Event_0
  (Utilities|Time|ClearandInvalidateTimerbyHandle (Variables|Default|GetEndRapidfireHandle)))

(event Custom|EndRapidFire
  (bind _owningchar (Variables|Default|GetOwningChar))
  (bind _speechrecognizer (Variables|/Game/Blueprints/Character/MuckenkolloseumChar.MuckenkolloseumChar_C|GetSpeechRecognizer _owningchar))
  (Variables|Default|SetisRapidFiring false)
  (Utilities|Time|ClearandInvalidateTimerbyHandle (Variables|Default|GetFireTimerHandle))
  (EventDispatchers|UnbindEventfromOnStartedSpeaking _speechrecognizer (delegate Custom|OnStartedSpeaking_Event_0))
  (EventDispatchers|UnbindEventfromOnStoppedSpeaking _speechrecognizer (delegate Custom|StopRapidfire))
  (Variables|/Game/Blueprints/Character/MuckenkolloseumChar.MuckenkolloseumChar_C|SetBlockSpeech (Variables|Default|GetOwningChar) false))

(event Custom|RapidFireTick
  (bind (_outhit _returnvalue) (Default|GetTargetedPosition (Variables|Default|GetOwningChar)))
  (CallFunction|RapidFireTickRMI (select _returnvalue (.Location (Collision|BreakHitResult _outhit)) (.TraceEnd (Collision|BreakHitResult _outhit)))))

(event EventTriggerWordSpoken
  (params (LookAtLocation :type Vector :default "0, 0, 0"))
  (Variables|/Game/Blueprints/Character/MuckenkolloseumChar.MuckenkolloseumChar_C|SetBlockSpeech (Variables|Default|GetOwningChar) true)
  (|CallParentFunction LookAtLocation))

(event EventAttachtoPlayer
  (params (OwningChar :type Muckenkolloseum%20Char%20Object%20Reference))
  (|CallParentFunction OwningChar)
  (Transformation|AttachComponentToComponent (Variables|/Script/Engine.Character|GetMesh OwningChar) "hand_rSocket" "SnapToTarget" "SnapToTarget" "KeepWorld" true))

(event EventTriggerWordSpokenClient
  (bind _owningchar (Variables|Default|GetOwningChar))
  (bind _speechrecognizer (Variables|/Game/Blueprints/Character/MuckenkolloseumChar.MuckenkolloseumChar_C|GetSpeechRecognizer _owningchar))
  (Utilities|FlowControl|Sequence
    (:then_0
      (EventDispatchers|AssignOnStartedSpeaking _speechrecognizer (delegate Custom|OnStartedSpeaking_Event_0))
      (EventDispatchers|BindEventtoOnStoppedSpeaking _speechrecognizer (delegate Custom|StopRapidfire))
      (Variables|Default|SetisRapidFiring true)
      (bind _returnvalue (Utilities|Time|SetTimerbyEvent (delegate Custom|RapidFireTick) (Variables|Default|GetInterval) true))
      (Variables|Default|SetFireTimerHandle _returnvalue))
    (:then_1
      (bind _returnvalue_2 (Utilities|Time|SetTimerbyEvent (delegate Custom|EndRapidFire) (Variables|Default|GetGraceperiod)))
      (Variables|Default|SetEndRapidfireHandle _returnvalue_2))))

(event EventEndPlay
  (params (EndPlayReason :type EEndPlayReason%20Enum :default "Destroyed"))
  (bind _owningchar (Variables|Default|GetOwningChar)
    (:then
      (Variables|/Game/Blueprints/Character/MuckenkolloseumChar.MuckenkolloseumChar_C|SetBlockSpeech _owningchar false))
    (:else)))

(fn ConstructionScript
  (|CallParentFunction))