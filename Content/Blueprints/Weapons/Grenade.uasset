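; Held grenade weapon that is thrown when its trigger word is spoken.
; It attaches to the character's right-hand socket and plays a hold montage on equip.
; On trigger it sets IsIgnited, spawns a ThrowableGrenade, launches it along the owner's forward vector pitched by Angle, plays the throw montage and destroys itself.
; LookAtLocation does not steer the throw, the targeted-arc logic is disconnected, and the IsIgnited RepNotify is empty.
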(event Custom|OnThrow
  (Animation|Montage|MontagePlay (Components|SkeletalMesh|GetAnimInstance (Variables|/Script/Engine.Character|GetMesh (Variables|Default|GetOwningChar))) "/Game/Meshes/Character/Character_throwGranate_Montage.Character_throwGranate_Montage" 1.0 "MontageLength" 0.0))

(event EventTriggerWordSpoken
  (params (LookAtLocation :type Vector :default "0, 0, 0"))
  (bind _owningchar (Variables|Default|GetOwningChar))
  (bind _owningchar_2 (Variables|Default|GetOwningChar))
  (|CallParentFunction LookAtLocation)
  (Variables|Default|SetisIgnited true)
  (bind _returnvalue (Game|SpawnActorfromClass "/Game/Blueprints/Weapons/ThrowableGrenade.ThrowableGrenade_C" (Transformation|GetActorTransform) "AlwaysSpawn" _owningchar_2 _owningchar_2))
  (Physics|AddImpulse (Variables|/Game/Blueprints/Weapons/ThrowableGrenade.ThrowableGrenade_C|GetSphere _returnvalue) (* (Math|Vector|RotateVectorAroundAxis (Transformation|GetActorForwardVector _owningchar) (Variables|Default|GetAngle) (Transformation|GetActorRightVector _owningchar)) (Variables|Default|GetThrowSpeed)) "None" true)
  (CallFunction|OnThrow)
  (Actor|DestroyActor))

(event EventEquip
  (|CallParentFunction)
  (Animation|Montage|MontagePlay (Components|SkeletalMesh|GetAnimInstance (Variables|/Script/Engine.Character|GetMesh (Variables|Default|GetOwningChar))) "/Game/Meshes/Character/Character_HoldGranate_Montage.Character_HoldGranate_Montage" 1.0 "MontageLength" 0.0))

(event EventAttachtoPlayer
  (params (OwningChar :type Muckenkolloseum%20Char%20Object%20Reference))
  (|CallParentFunction OwningChar)
  (Transformation|AttachComponentToComponent (Variables|/Script/Engine.Character|GetMesh OwningChar) "hand_rSocket" "SnapToTarget" "SnapToTarget" "KeepWorld" true)
  (Transformation|SetRelativeLocation (Variables|Default|GetDefaultSceneRoot) "1.000000,-1.000000, 0" false false))

(fn ConstructionScript
  (|CallParentFunction))

(fn OnRepIsIgnited)