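; Rapid-fire weapon bullet that explodes when destroyed, dealing radial damage.
; On BeginPlay it applies its configured scale, and the server destroys it after a short lifetime.
; Server-side overlaps with anything except the owning MuckenkolloseumChar print the hit actor's name and destroy the bullet.
; EndPlay applies full damage within the explosion radius and spawns the explosion effect, with no server check.
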(event Collision|EventActorBeginOverlap
  (params (OtherActor :type Actor%20Object%20Reference))
  (if (Networking|IsServer)
    (bind _asmuckenkolloseum_char (Utilities|Casting|CastToMuckenkolloseumChar OtherActor)
      (:then
        (if (!= _asmuckenkolloseum_char (Components|GetOwner))
          (Development|PrintString (Utilities|GetDisplayName OtherActor) true true "(R=1.000000,G=0.092550,B=0.000000,A=1.000000)" :!label _label)
          (Actor|DestroyActor)))
      (:CastFailed
        (goto _label)))))

(event EventBeginPlay
  (bind _scale (Variables|Default|GetScale))
  (Transformation|SetActorScale3D (Math|Vector|MakeVector _scale _scale _scale))
  (if (Networking|IsServer)
    (Utilities|FlowControl|Delay 4.0)
    (Actor|DestroyActor)))

(event EventEndPlay
  (params (EndPlayReason :type EEndPlayReason%20Enum :default "Destroyed"))
  (bind _returnvalue (Transformation|GetActorLocation))
  (Game|Damage|ApplyRadialDamage (Variables|Default|GetDamage) _returnvalue (Variables|Default|GetExplosionRadius) "/Game/Blueprints/Damage/ExplosionDamage.ExplosionDamage_C" 0 self 0 true "ECC_Visibility")
  (Game|SpawnActorfromClass "/Game/StarterContent/Blueprints/Blueprint_Effect_Explosion.Blueprint_Effect_Explosion_C" (Math|Transform|MakeTransform _returnvalue "0, 0, 0" "4.000000,4.000000,4.000000") "AlwaysSpawn" 0 0))

(fn ConstructionScript)