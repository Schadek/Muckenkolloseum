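; Weapon pickup actor that displays a spinning weapon of a configurable class and gives it to a player character who touches it.
; BeginPlay spawns the weapon through a child actor component and scales it by its own PickupScale.
; On sphere overlap, the authority attaches that same weapon instance to the character, then calls DeactivationRMI to stop rotation, particles and sphere collision.
; Nothing here reactivates the pickup afterwards.
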(event OnComponentBeginOverlap(Sphere)
  (params (OverlappedComponent :type Primitive%20Component%20Object%20Reference) (OtherActor :type Actor%20Object%20Reference) (OtherComp :type Primitive%20Component%20Object%20Reference) (OtherBodyIndex :type Integer) (bFromSweep :type Boolean) (SweepResult :type Hit%20Result%20Structure%20%28by%20ref%29))
  (bind _asmuckenkolloseum_char (Utilities|Casting|CastToMuckenkolloseumChar OtherActor))
  (Networking|SwitchHasAuthority
    (:Authority
      (bind _asbase_weapon (Utilities|Casting|CastToBaseWeapon (Variables|/Script/Engine.ChildActorComponent|GetChildActor (Variables|Default|GetChildActor))))
      (Default|AttachtoPlayer _asbase_weapon _asmuckenkolloseum_char)
      (CallFunction|DeactivationRMI false))))

(event Custom|DeactivationRMI
  (params (isActive :type Boolean))
  (CallFunction|SetActive isActive))

(event EventBeginPlay
  (bind _childactor (Variables|Default|GetChildActor))
  (ChildActorComponent|SetChildActorClass _childactor (Variables|Default|GetWeaponClass))
  (bind _asbase_weapon (Utilities|Casting|CastToBaseWeapon (Variables|/Script/Engine.ChildActorComponent|GetChildActor _childactor)))
  (Transformation|SetWorldScale3D (Variables|Default|GetChildActor) (Math|Vector|MakeVector (Variables|/Game/Blueprints/Weapons/BaseWeapon.BaseWeapon_C|GetPickupScale _asbase_weapon) (Variables|/Game/Blueprints/Weapons/BaseWeapon.BaseWeapon_C|GetPickupScale _asbase_weapon) (Variables|/Game/Blueprints/Weapons/BaseWeapon.BaseWeapon_C|GetPickupScale _asbase_weapon))))

(event EventTick
  (params (DeltaSeconds :type Float%20%28single-precision%29))
  (if (Variables|Default|GetisActive)
    (Transformation|AddWorldRotation (Variables|Default|GetChildActor) (* "0,60.000000, 0" DeltaSeconds) false false)))

(fn ConstructionScript)

(fn SetActive
  (params (isActive :type Boolean))
  (bind _output_get (Variables|Default|SetisActive isActive))
  (Components|Activation|SetActive (Variables|Default|GetParticleSystem) _output_get true)
  (Collision|SetCollisionEnabled (Variables|Default|GetSphere) (select _output_get "QueryOnly" "NoCollision")))