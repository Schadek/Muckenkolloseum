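; Game mode for Muckenkolloseum that scores kills and supplies respawn settings.
; On player death, the killer's MuckenkolloseumPlayerStateBP gains a point and the victim's loses one.
; The victim's penalty runs only after the killer's PlayerState cast succeeds.
; Respawn functions return a constant delay and a fixed spawn point just above the world origin, regardless of character.
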(event Custom|PlayerDied
  (params (Character :type Muckenkolloseum%20Char%20Object%20Reference) (KillerInstigator :type Player%20Controller%20Object%20Reference))
  (bind _asmuckenkolloseum_player_state_bp (Utilities|Casting|CastToMuckenkolloseumPlayerStateBP (Variables|/Script/Engine.Controller|GetPlayerState KillerInstigator)))
  (Math|Integer|IncrementInt (Variables|/Game/Gamemodes/MuckenkolloseumPlayerStateBP.MuckenkolloseumPlayerStateBP_C|GetPoints _asmuckenkolloseum_player_state_bp)
    (:%20%20
      (bind _asmuckenkolloseum_player_state_bp_2 (Utilities|Casting|CastToMuckenkolloseumPlayerStateBP (Variables|/Script/Engine.Controller|GetPlayerState (.AsPlayer%20Controller (Utilities|Casting|CastToPlayerController (Pawn|GetController Character))))))
      (Math|Integer|DecrementInt (Variables|/Game/Gamemodes/MuckenkolloseumPlayerStateBP.MuckenkolloseumPlayerStateBP_C|GetPoints _asmuckenkolloseum_player_state_bp_2)))))

(event EventBeginPlay)

(event EventTick
  (params (DeltaSeconds :type Float%20%28single-precision%29)))

(fn ConstructionScript)

(fn GetRespawnTimer
  (params (Character :type Muckenkolloseum%20Char%20Object%20Reference))
  (return 8.0))

(fn GetRespawnPoint
  (params (Character :type Muckenkolloseum%20Char%20Object%20Reference))
  (return (Math|Vector|MakeVector 0.0 0.0 2e+02)))