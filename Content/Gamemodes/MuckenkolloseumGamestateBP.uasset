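; Game state for the Muckenkolloseum game mode that runs a timed match and shows the in-game UI.
; On BeginPlay it adds the IngameUI widget for player controller 0, then sets MatchEnd from the current game time plus MatchDuration.
; MatchEnd's RepNotify flags the match as running.
; GetRemainingMatchTime returns MatchEnd minus server world time, along with that flag.
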(event Custom|StartGame
  (Variables|Default|SetMatchEnd (+ (Utilities|Time|GetTimeSeconds) (Variables|Default|GetMatchDuration))))

(event EventBeginPlay
  (bind _returnvalue (UserInterface|CreateWidget "/Game/UI/IngameUI.IngameUI_C" (Game|GetPlayerController 0)))
  (UserInterface|Viewport|AddtoViewport _returnvalue 0)
  (CallFunction|StartGame))

(fn ConstructionScript)

(fn GetRemainingMatchTime
  (return (- (Variables|Default|GetMatchEnd) (GameState|GetServerWorldTimeSeconds)) (Variables|Default|GetMatchRunning)))

(fn OnRepMatchEnd
  (Variables|Default|SetMatchRunning true))