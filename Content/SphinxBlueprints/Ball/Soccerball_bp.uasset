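; Soccer ball actor that randomly takes on a red or blue team colour when constructed.
; The construction script calls RandomColour, which flips a random bool, sets the matching Red and Blue flags, and applies the corresponding material to the static mesh.
; The event graph holds only disabled default events, so all logic runs at construction.
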(event EventBeginPlay)

(event Collision|EventActorBeginOverlap
  (params (OtherActor :type Actor%20Object%20Reference)))

(event EventTick
  (params (DeltaSeconds :type Float%20%28single-precision%29)))

(fn ConstructionScript
  (CallFunction|RandomColour))

(fn RandomColour
  (if (Math|Random|RandomBool)
    (Variables|Default|Setblue false)
    (Variables|Default|Setred true)
    (Rendering|Material|SetMaterial (Variables|Debug|GetStaticMeshComponent) 0 "/Game/StarterContent/Materials/Colours/Red_Mat.Red_Mat")
    (else
      (Variables|Default|Setblue true)
      (Variables|Default|Setred false)
      (Rendering|Material|SetMaterial (Variables|Debug|GetStaticMeshComponent) 0 "/Game/StarterContent/Materials/Colours/Blue_Mat.Blue_Mat"))))